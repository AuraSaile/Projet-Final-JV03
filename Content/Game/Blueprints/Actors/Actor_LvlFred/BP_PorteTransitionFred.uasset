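; Transition door actor that takes the player to the level Lvl_02_FrédéricBilodeau when interacted with.
; On Interact, it fades the camera to black, waits for the fade to finish, then opens the level.
; A sphere trigger shows its interaction widget while the third-person character overlaps it.
; Each tick, the widget component rotates to face the player character.
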(event `/Game/Game/Blueprints/Interfaces/BPI_Interact.Interact`
  (params (Actor :type "Actor Object Reference"))
  ; Changer de niveau
  (`PlayerCameraManager.StartCameraFade` (`GameplayStatics.GetPlayerCameraManager` 0) 0.0 1.0 1.0 (struct :`A` 1.0) false true)
  (`KismetSystemLibrary.Delay` 1.0)
  (`GameplayStatics.OpenLevelBySoftObjectPtr` "/Game/Game/Maps/Lvl_02_FrédéricBilodeau.Lvl_02_FrédéricBilodeau"))

(event `self.Sphere.OnComponentBeginOverlap`
  (params (OverlappedComponent :type "PrimitiveComponent Object Reference") (OtherActor :type "Actor Object Reference") (OtherComp :type "PrimitiveComponent Object Reference") (OtherBodyIndex :type Integer) (bFromSweep :type Boolean) (SweepResult :type "HitResult Structure (by ref)"))
  ; Apparition WBP_Interact
  (cast `/Game/Game/Blueprints/Pawns_Characters/Player/BP_ThirdPersonCharacter` OtherActor)
  (`SceneComponent.SetVisibility` (`self.Widget`) true false))

(event `self.Sphere.OnComponentEndOverlap`
  (params (OverlappedComponent :type "PrimitiveComponent Object Reference") (OtherActor :type "Actor Object Reference") (OtherComp :type "PrimitiveComponent Object Reference") (OtherBodyIndex :type Integer))
  ; Enlèvement WBP_Interact
  (cast `/Game/Game/Blueprints/Pawns_Characters/Player/BP_ThirdPersonCharacter` OtherActor)
  (`SceneComponent.SetVisibility` (`self.Widget`) false false))

(event `self.ReceiveTick`
  (params (DeltaSeconds :type "Float (single-precision)"))
  ; Faire face au joueur
  (`SceneComponent.K2_SetWorldRotation` (`self.Widget`) (`KismetMathLibrary.FindLookAtRotation` (`SceneComponent.K2_GetComponentLocation` (`self.Widget`)) (`self.K2_GetActorLocation` (`GameplayStatics.GetPlayerCharacter` 0))) false false))

(fn `UserConstructionScript`)