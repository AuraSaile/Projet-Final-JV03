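; BP_PorteAntoine is an interactable sci-fi door actor that opens in two halves, then removes itself from the level.
; Interact stores each panel's relative transform, then a timeline raises the upper panel while, one second later, another lowers the bottom panel.
; Timeline values offset each panel's relative Z.
; A five-second Delay, triggered from the lower timeline's Update, destroys the actor.
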(event `/Game/Game/Blueprints/Interfaces/BPI_Interact.Interact`
  (params (Actor :type "Actor Object Reference"))
  (bind _startlocationbas (`self.StartLocationBas`))
  (bind _startlocationhaut (`self.StartLocationHaut`))
  ; Animation Complète de ma porte
  (`|ExecutionSequence`
    (:`then_0`
      (set `self.StartLocationHaut` (`SceneComponent.GetRelativeTransform` (`self.mScifi_Door01Up_M_door01_Dark_0`)))
      (bind (_direction _animationhaut) (`Timeline|AnimationHaut`)
        (:`Update`
          (`SceneComponent.K2_SetRelativeLocation` (`self.mScifi_Door01Up_M_door01_Dark_0`) (`KismetMathLibrary.MakeVector` (.x (.location _startlocationhaut)) (.y (.location _startlocationhaut)) (+ (* _animationhaut 100.0) (.z (.location _startlocationhaut)))) false false))))
    (:`then_1`
      (set `self.StartLocationBas` (`SceneComponent.GetRelativeTransform` (`self.mScifi_Door01Down_M_door01_Dark_0`)))
      (`KismetSystemLibrary.Delay` 1.0)
      (bind (_direction_2 _newtrack_0) (`Timeline|AnimationBas`)
        (:`Update`
          (`SceneComponent.K2_SetRelativeLocation` (`self.mScifi_Door01Down_M_door01_Dark_0`) (`KismetMathLibrary.MakeVector` (.x (.location _startlocationbas)) (.y (.location _startlocationbas)) (+ (* _newtrack_0 -50.0) (.z (.location _startlocationbas)))) false false)
          (`KismetSystemLibrary.Delay` 5.0)
          (`self.K2_DestroyActor`))))))

(fn `UserConstructionScript`)