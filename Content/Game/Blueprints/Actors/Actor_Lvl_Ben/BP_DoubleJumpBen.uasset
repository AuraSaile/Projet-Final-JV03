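; Interactable double-jump pickup that sets the player character's JumpMaxCount to two and plays a sound.
; On Interact it hides the cactus mesh, disables actor collision and shows the WBP_DoubleJump notice briefly, then restores mesh and collision after a longer delay.
; A sphere overlap toggles the interact prompt widget for the player character.
; The jump upgrade is never reverted here.
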(event `/Game/Game/Blueprints/Interfaces/BPI_Interact.Interact`
  (params (Actor :type "Actor Object Reference"))
  ; Double Jump
  (bind _asbp_third_person_character (cast `/Game/Game/Blueprints/Pawns_Characters/Player/BP_ThirdPersonCharacter` (`GameplayStatics.GetPlayerCharacter` 0)))
  (set `Character.JumpMaxCount` 2 _asbp_third_person_character)
  (`GameplayStatics.PlaySound2D` "/Game/Game/Audio/SFX/SFX_DoubleJump.SFX_DoubleJump" 1.0 1.0 0.0 null null)
  (`SceneComponent.SetVisibility` (`self.cactus_small_B`) false false)
  (`self.SetActorEnableCollision` (`ActorComponent.GetOwner` (`self.cactus_small_B`)) false)
  (bind _returnvalue (`|CreateWidget` "/Game/Game/UI/WBP_DoubleJump.WBP_DoubleJump_C"))
  (bind _output_get (set `self.DoubleJumpWBP_Ref` _returnvalue))
  (`UserWidget.AddToViewport` _output_get 1)
  (`|ExecutionSequence`
    (:`then_0`
      (`KismetSystemLibrary.Delay` 2.0)
      (`Widget.RemoveFromParent` (`self.DoubleJumpWBP_Ref`)))
    (:`then_1`
      (`KismetSystemLibrary.Delay` 4.0)
      (`SceneComponent.SetVisibility` (`self.cactus_small_B`) true false)
      (`self.SetActorEnableCollision` (`ActorComponent.GetOwner` (`self.cactus_small_B`)) true))))

(event `self.sphereCollider.OnComponentBeginOverlap`
  (params (OverlappedComponent :type "PrimitiveComponent Object Reference") (OtherActor :type "Actor Object Reference") (OtherComp :type "PrimitiveComponent Object Reference") (OtherBodyIndex :type Integer) (bFromSweep :type Boolean) (SweepResult :type "HitResult Structure (by ref)"))
  ; Apparition WBP_Interact
  (cast `/Game/Game/Blueprints/Pawns_Characters/Player/BP_ThirdPersonCharacter` OtherActor)
  (`SceneComponent.SetVisibility` (`self.Widget`) true false))

(event `self.sphereCollider.OnComponentEndOverlap`
  (params (OverlappedComponent :type "PrimitiveComponent Object Reference") (OtherActor :type "Actor Object Reference") (OtherComp :type "PrimitiveComponent Object Reference") (OtherBodyIndex :type Integer))
  ; Enlèvement WBP_Interact
  (cast `/Game/Game/Blueprints/Pawns_Characters/Player/BP_ThirdPersonCharacter` OtherActor)
  (`SceneComponent.SetVisibility` (`self.Widget`) false false))

(fn `UserConstructionScript`)