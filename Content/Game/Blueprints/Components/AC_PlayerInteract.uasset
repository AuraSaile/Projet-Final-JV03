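; Player interaction component that finds the interactable actor the player's camera is looking at.
; On BeginPlay it caches the owning BP_ThirdPersonCharacter.
; Its Linetrace function traces on the Visibility channel from the follow camera along its forward vector for a given length, returning the hit actor only if it implements BPI_Interact.
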(event `self.ReceiveBeginPlay`
  ; Set de la variable Bp_ThirdPerson Ref
  (bind _asbp_third_person_character (cast `/Game/Game/Blueprints/Pawns_Characters/Player/BP_ThirdPersonCharacter` (`self.GetOwner`)))
  (set `self.BP_ThirdPersonRef` _asbp_third_person_character))

(fn `Linetrace`
  (params (Lenght :type "Float (double-precision)"))
  (returns (HitActor :type "Actor Object Reference"))
  (bind _followcamera (`/Game/Game/Blueprints/Pawns_Characters/Player/BP_ThirdPersonCharacter.FollowCamera` (`self.BP_ThirdPersonRef`)))
  (bind _returnvalue (`SceneComponent.K2_GetComponentLocation` _followcamera))
  ; Ligne pour l'interact
  (bind _outhit (`KismetSystemLibrary.LineTraceSingle` _returnvalue (+ _returnvalue (* (`SceneComponent.GetForwardVector` _followcamera) Lenght)) "TraceTypeQuery1"))
  (bind (_bblockinghit _binitialoverlap _time _distance _location _impactpoint _normal _impactnormal _physmat _hitactor) (`GameplayStatics.BreakHitResult` _outhit))
  (if (and (`KismetSystemLibrary.IsValid` _hitactor) (`KismetSystemLibrary.DoesImplementInterface` _hitactor "/Game/Game/Blueprints/Interfaces/BPI_Interact.BPI_Interact_C"))
    (return _hitactor)
    (else
      (return null))))